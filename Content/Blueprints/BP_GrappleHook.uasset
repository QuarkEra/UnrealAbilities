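; Short-lived grapple hook projectile that pulls its owning BP_PlayerCharacter toward whatever it hits.
; On overlapping anything but a player character, it stops and launches the owner along the clamped player-to-hook vector.
; A hook below the player replaces that vector's vertical part with a fixed downward offset, despite the Zboost name.
; When the player is already moving fast, current velocity is subtracted from the additive launch.
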(event `self.ReceiveBeginPlay`
  (`self.SetLifeSpan` 0.35))

(event `self.Sphere.OnComponentBeginOverlap`
  (params (OverlappedComponent :type "PrimitiveComponent Object Reference") (OtherActor :type "Actor Object Reference") (OtherComp :type "PrimitiveComponent Object Reference") (OtherBodyIndex :type Integer) (bFromSweep :type Boolean) (SweepResult :type "HitResult Structure (by ref)"))
  (bind (_returnvalue_x _returnvalue_y _returnvalue_z) (`KismetMathLibrary.BreakVector` (`self.K2_GetActorLocation`)))
  (cast `/Game/Blueprints/BP_PlayerCharacter` OtherActor
    (:`CastFailed`
      (`ProjectileMovementComponent.StopSimulating` (`self.ProjectileMovement`) SweepResult)
      (bind _asbp_player_character (cast `/Game/Blueprints/BP_PlayerCharacter` (`self.GetOwner`)))
      (bind (_returnvalue_x_2 _returnvalue_y_2 _returnvalue_z_2) (`KismetMathLibrary.BreakVector` (`self.K2_GetActorLocation` _asbp_player_character)))
      (if (< _returnvalue_z _returnvalue_z_2)
        (set `self.Zboost` (+ _returnvalue_z 500.0))
        (bind _returnvalue (`self.GetVelocity` _asbp_player_character))
        (if (> (`KismetMathLibrary.VSize` _returnvalue) 1000.0)
          (bind _returnvalue_2 (`KismetMathLibrary.ClampVectorSize` (- (`KismetMathLibrary.MakeVector` _returnvalue_x _returnvalue_y _returnvalue_z) (`KismetMathLibrary.MakeVector` _returnvalue_x_2 _returnvalue_y_2 (`self.Zboost`))) 1000.0 2000.0))
          (`Character.LaunchCharacter` _asbp_player_character (- _returnvalue_2 _returnvalue) false false)
          (else
            (`Character.LaunchCharacter` _asbp_player_character _returnvalue_2 false false)))
        (else
          (bind _returnvalue_3 (`self.GetVelocity` _asbp_player_character))
          (if (> (`KismetMathLibrary.VSize` _returnvalue_3) 1000.0)
            (bind _returnvalue_4 (`KismetMathLibrary.ClampVectorSize` (- (`self.K2_GetActorLocation`) (`self.K2_GetActorLocation` _asbp_player_character)) 1000.0 2000.0))
            (`Character.LaunchCharacter` _asbp_player_character (- _returnvalue_4 _returnvalue_3) false false)
            (else
              (`Character.LaunchCharacter` _asbp_player_character _returnvalue_4 false false))))))))

(fn `UserConstructionScript`)