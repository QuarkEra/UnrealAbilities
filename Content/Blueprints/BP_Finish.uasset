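; BP_Finish is the level's finish-line actor, triggered when the player character overlaps its box.
; On BeginPlay it caches the first AmbientSound found in the level as the background music.
; The first player overlap, guarded by a DoOnce, records the finish time through the player's UI and fades out the music.
; After a short delay it destroys the player character if still valid.
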(event `self.ReceiveBeginPlay`
  (bind _outactors (`GameplayStatics.GetAllActorsOfClass` "/Script/Engine.AmbientSound"))
  (if (`KismetArrayLibrary.Array_IsValidIndex` _outactors)
    (set `self.BGM` (`|GetArrayItem` _outactors))))

(event `self.Box.OnComponentBeginOverlap`
  (params (OverlappedComponent :type "PrimitiveComponent Object Reference") (OtherActor :type "Actor Object Reference") (OtherComp :type "PrimitiveComponent Object Reference") (OtherBodyIndex :type Integer) (bFromSweep :type Boolean) (SweepResult :type "HitResult Structure (by ref)"))
  (bind _asbp_player_character (cast `/Game/Blueprints/BP_PlayerCharacter` OtherActor))
  (`/Engine/EditorBlueprintResources/StandardMacros.DoOnce` false
    (:`Completed`
      (`/Game/Blueprints/UI/WB_UI.SetFinishTime` (`/Game/Blueprints/BP_PlayerCharacter.UI` _asbp_player_character))
      (`AudioComponent.FadeOut` (`AmbientSound.AudioComponent` (`self.BGM`)) 1.0 0.0 "Linear")
      (`KismetSystemLibrary.Delay` 5.0)
      (`/Engine/EditorBlueprintResources/StandardMacros.IsValid` _asbp_player_character
        (:`Is Valid`
          (`self.K2_DestroyActor` _asbp_player_character))))))

(fn `UserConstructionScript`)