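; Game mode that handles player respawning and the end-of-mission score screen.
; On BeginPlay and after each respawn it binds to the player character's destroyed event and sets game-only input.
; When the character is destroyed, a short delay precedes spawning and possessing a replacement at SpawnTransform.
; MissionComplete records the finish time, swaps the player UI for WB_ScoreScreen, switches to UI-only input and pauses the game.
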(event `CE_Respawn`
  (bind _returnvalue (`GameplayStatics.GetPlayerController` 0))
  (bind _asbp_player_character (cast `/Game/Blueprints/BP_PlayerCharacter` (`GameplayStatics.GetPlayerCharacter` 0) :!label _label))
  (add `self.OnDestroyed` _asbp_player_character (delegate `CE_OnDestroyed`))
  (`WidgetBlueprintLibrary.SetInputMode_GameOnly` _returnvalue)
  (set `PlayerController.bShowMouseCursor` false _returnvalue))

(event `self.ReceiveBeginPlay`
  (goto _label))

(event `CE_OnDestroyed` :!signature `self.OnDestroyed`
  (params (DestroyedActor :type "Actor Object Reference"))
  (`KismetSystemLibrary.Delay` 0.2)
  (bind _returnvalue (`|SpawnActorFromClass` "/Game/Blueprints/BP_PlayerCharacter.BP_PlayerCharacter_C" (`self.Spawn Transform`) "Undefined" "MultiplyWithRoot" null null))
  (`Controller.Possess` (`GameplayStatics.GetPlayerController` 0) _returnvalue)
  (`self.CE_Respawn`))

(fn `MissionComplete`
  (bind _returnvalue (`GameplayStatics.GetPlayerController` 0))
  (bind _asbp_player_character (cast `/Game/Blueprints/BP_PlayerCharacter` (`GameplayStatics.GetPlayerCharacter` 0)))
  (`/Game/Blueprints/UI/WB_UI.SetFinishTime` (`/Game/Blueprints/BP_PlayerCharacter.UI` _asbp_player_character))
  (`/Game/Blueprints/BP_PlayerCharacter.RemoveUI` _asbp_player_character)
  (bind _returnvalue_2 (`|CreateWidget` "/Game/Blueprints/UI/WB_ScoreScreen.WB_ScoreScreen_C"))
  (`UserWidget.AddToViewport` _returnvalue_2 0)
  (`WidgetBlueprintLibrary.SetInputMode_UIOnlyEx` _returnvalue _returnvalue_2 "LockInFullscreen")
  (bind _output_get (set `PlayerController.bShowMouseCursor` true _returnvalue))
  (`GameplayStatics.SetGamePaused` _output_get))

(fn `UserConstructionScript`)