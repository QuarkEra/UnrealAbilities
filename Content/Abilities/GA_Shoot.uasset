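; GA_Shoot is a gameplay ability that fires a hitscan shot to destroy BP_Target actors.
; On activation it commits, then line-traces on the Camera channel from the player camera along its forward vector, leaving persistent debug lines.
; A valid target hit is destroyed with a 2D sound before the ability ends.
; EndAbility is only called on that hit path, so a miss leaves the ability active.
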(event `self.K2_ActivateAbility`
  (bind _transformcomponent (`PlayerCameraManager.TransformComponent` (`GameplayStatics.GetPlayerCameraManager` 0)))
  (bind _returnvalue (`SceneComponent.K2_GetComponentLocation` _transformcomponent))
  (`parent.K2_ActivateAbility`)
  (`self.K2_CommitAbility`)
  (bind _outhit (`KismetSystemLibrary.LineTraceSingle` :`Start` _returnvalue :`End` (+ _returnvalue (* (`KismetMathLibrary.GetForwardVector` (`SceneComponent.K2_GetComponentRotation` _transformcomponent)) (`self.TraceLength`))) :`TraceChannel` "TraceTypeQuery2" :`bTraceComplex` true :`DrawDebugType` "Persistent"))
  (bind _asbp_target (cast `/Game/Blueprints/BP_Target` (`.HitActor` (`GameplayStatics.BreakHitResult` _outhit))))
  (`/Engine/EditorBlueprintResources/StandardMacros.IsValid` _asbp_target
    (:`Is Valid`
      (`Actor.K2_DestroyActor` _asbp_target)
      (`GameplayStatics.PlaySound2D` "/Engine/VREditor/Sounds/VR_ungrab.VR_ungrab" 1.0 1.0 0.0 null null)
      (`self.K2_EndAbility`))))