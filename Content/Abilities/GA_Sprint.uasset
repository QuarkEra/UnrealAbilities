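; Gameplay ability that makes BP_PlayerCharacter sprint.
; On activation it commits, doubles the character's max walk speed, starts a wait for removal of the Ability.Sprint tag, and applies GE_Sprint to the owner.
; When the tag is removed, it sets walk speed to a hardcoded default rather than the saved original and ends the ability.
; OnEndAbility is unused, so speed resets only through that tag-removal path.
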(event `self.K2_ActivateAbility`
  (bind _asbp_player_character (cast `/Game/Blueprints/BP_PlayerCharacter` (`self.GetOwningActorFromActorInfo`)))
  (`self.K2_CommitAbility`)
  (bind _charactermovement (`Character.CharacterMovement` _asbp_player_character))
  (set `CharacterMovementComponent.MaxWalkSpeed` (* (`CharacterMovementComponent.MaxWalkSpeed` _charactermovement) 2.0) _charactermovement)
  (`AbilityTask_WaitGameplayTagRemoved.WaitGameplayTagRemove` (struct :`TagName` "Ability.Sprint") null true
    (:`then`
      (`self.BP_ApplyGameplayEffectToOwner` "/Game/Abilities/GE_Sprint.GE_Sprint_C"))
    (:`Removed`
      (set `CharacterMovementComponent.MaxWalkSpeed` 600.0 _charactermovement)
      (`self.K2_EndAbility`))))