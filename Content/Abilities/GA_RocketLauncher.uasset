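; GA_RocketLauncher is a Gameplay Ability that fires a BP_Bouncer actor from the player character.
; On activation it casts the avatar's owning actor to BP_PlayerCharacter, commits the ability, spawns the bouncer and ends immediately.
; The spawn uses the character's location and the first player's camera manager rotation, always spawns despite collisions, and sets the character as Owner and Instigator.
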(event `self.K2_ActivateAbility`
  (`parent.K2_ActivateAbility`)
  (bind _asbp_player_character (cast `/Game/Blueprints/BP_PlayerCharacter` (`self.GetOwningActorFromActorInfo`)))
  (`self.K2_CommitAbility`)
  (`|SpawnActorFromClass` "/Game/Blueprints/BP_Bouncer.BP_Bouncer_C" (`KismetMathLibrary.MakeTransform` (`Actor.K2_GetActorLocation` _asbp_player_character) (`SceneComponent.K2_GetComponentRotation` (`PlayerCameraManager.TransformComponent` (`GameplayStatics.GetPlayerCameraManager` 0)))) "AlwaysSpawn" "MultiplyWithRoot" _asbp_player_character _asbp_player_character)
  (`self.K2_EndAbility`))