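; Gameplay ability that lets the player character wall run when its WallJumpOverlapper detects an overlapping actor.
; It commits, applies GE_WallRun, lowers gravity and launches the character with its horizontal velocity plus the first overlapped actor's flattened right vector, zeroing vertical speed.
; The effect's lifetime drives the run: its removal restores normal gravity and ends the ability.
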(event `self.K2_ActivateAbility`
  (bind _asbp_player_character (cast `/Game/Blueprints/BP_PlayerCharacter` (`self.GetOwningActorFromActorInfo`)))
  (bind _overlappingactors (`PrimitiveComponent.GetOverlappingActors` (`/Game/Blueprints/BP_PlayerCharacter.WallJumpOverlapper` _asbp_player_character) "/Script/Engine.Actor"))
  (if (> (`KismetArrayLibrary.Array_Length` _overlappingactors) 0)
    (`self.K2_CommitAbility`)
    (bind _returnvalue (`self.BP_ApplyGameplayEffectToOwner` "/Game/Abilities/GE_WallRun.GE_WallRun_C"))
    (bind _charactermovement (`Character.CharacterMovement` _asbp_player_character))
    (set `CharacterMovementComponent.GravityScale` 0.33 _charactermovement)
    (bind (_returnvalue_x _returnvalue_y) (`KismetMathLibrary.BreakVector` (`Actor.GetActorRightVector` (`|GetArrayItem` _overlappingactors))))
    (bind (_velocity_x _velocity_y) (`KismetMathLibrary.BreakVector` (`MovementComponent.Velocity` _charactermovement)))
    (`Character.LaunchCharacter` _asbp_player_character (+ (`KismetMathLibrary.MakeVector` _returnvalue_x _returnvalue_y) (`KismetMathLibrary.MakeVector` _velocity_x _velocity_y)) true true)
    (`AbilityTask_WaitGameplayEffectRemoved.WaitForGameplayEffectRemoved` _returnvalue
      (:`OnRemoved`
        (set `CharacterMovementComponent.GravityScale` 1.0 _charactermovement)
        (`self.K2_EndAbility`)
        (set `CharacterMovementComponent.GravityScale` 1.0 _charactermovement)))))