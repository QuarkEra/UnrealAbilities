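; GA_Jump is a Gameplay Ability that gives BP_PlayerCharacter a jump with a bunny-hop style air-strafe combo.
; When turning and strafing point the same way, it launches the character upward and along its velocity, with the directional boost scaled by HopCount.
; Each hop increments that count and restarts a short ClearJumpCombo timer on the character.
; Otherwise it performs a normal Jump, and the ability ends immediately either way.
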(event `self.K2_ActivateAbility`
  (bind _asbp_player_character (cast `/Game/Blueprints/BP_PlayerCharacter` (`self.GetOwningActorFromActorInfo`)))
  (`self.K2_CommitAbility`)
  (if (or (and (`/Game/Blueprints/BP_PlayerCharacter.TurningRight` _asbp_player_character) (`/Game/Blueprints/BP_PlayerCharacter.StrafingRight` _asbp_player_character)) (and (`/Game/Blueprints/BP_PlayerCharacter.TurningLeft` _asbp_player_character) (`/Game/Blueprints/BP_PlayerCharacter.StrafingLeft` _asbp_player_character)))
    (`Character.LaunchCharacter` _asbp_player_character (+ (* (`KismetMathLibrary.Normal` (`Actor.GetVelocity` _asbp_player_character)) (* (`self.LaunchForce`) (`/Game/Blueprints/BP_PlayerCharacter.HopCount` _asbp_player_character))) (* (`Actor.GetActorUpVector` _asbp_player_character) (`self.JumpForce`))) false false)
    (`/Engine/EditorBlueprintResources/StandardMacros.IncrementInt` (`/Game/Blueprints/BP_PlayerCharacter.HopCount` _asbp_player_character)
      (:`  `
        (`KismetSystemLibrary.K2_SetTimer` _asbp_player_character "ClearJumpCombo" 1.0)))
    (else
      (`Character.Jump` _asbp_player_character)))
  (`self.K2_EndAbility`))