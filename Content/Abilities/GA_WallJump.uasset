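; GA_WallJump is a Gameplay Ability that lets BP_PlayerCharacter jump off a wall.
; On activation, it proceeds only if the character's WallJumpOverlapper overlaps at least one actor, then commits the ability.
; It resets gravity scale, calls Jump and launches the character along its forward and up vectors, overriding only vertical velocity, then ends.
; When nothing overlaps, the graph never calls EndAbility.
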(event `self.K2_ActivateAbility`
  (bind _asbp_player_character (cast `/Game/Blueprints/BP_PlayerCharacter` (`self.GetOwningActorFromActorInfo`)))
  (if (> (`KismetArrayLibrary.Array_Length` (`PrimitiveComponent.GetOverlappingActors` (`/Game/Blueprints/BP_PlayerCharacter.WallJumpOverlapper` _asbp_player_character) "/Script/Engine.Actor")) 0)
    (`self.K2_CommitAbility`)
    (set `CharacterMovementComponent.GravityScale` 1.0 (`Character.CharacterMovement` _asbp_player_character))
    (`Character.Jump` _asbp_player_character)
    (`Character.LaunchCharacter` _asbp_player_character (+ (* (`Actor.GetActorForwardVector` _asbp_player_character) (`self.LaunchForce`)) (* (`Actor.GetActorUpVector` _asbp_player_character) (`self.JumpForce`))) false true)
    (`self.K2_EndAbility`)))