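; GA_Slide is a Gameplay Ability that makes the player character slide when activated on the ground.
; It commits, lowers ground friction, crouches, launches the character forward by Speed and widens the camera manager's default FOV.
; GE_Slide is applied while a task waits for removal of the Ability.Slide tag, which resets friction, restores FOV, uncrouches and ends the ability.
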(event `self.K2_ActivateAbility`
  (bind _returnvalue (`GameplayStatics.GetPlayerCameraManager` 0))
  (bind _defaultfov (`PlayerCameraManager.DefaultFOV` _returnvalue))
  (bind _asbp_player_character (cast `/Game/Blueprints/BP_PlayerCharacter` (`self.GetOwningActorFromActorInfo`)))
  (if (`NavMovementComponent.IsMovingOnGround` (`Character.CharacterMovement` _asbp_player_character))
    (`self.K2_CommitAbility`)
    (set `CharacterMovementComponent.GroundFriction` 0.5 (`Character.CharacterMovement` _asbp_player_character))
    (`Character.Crouch` _asbp_player_character)
    (`Character.LaunchCharacter` _asbp_player_character (* (`Actor.GetActorForwardVector` _asbp_player_character) (`self.Speed`)) false false)
    (set `self.Default FOV` _defaultfov)
    (set `PlayerCameraManager.DefaultFOV` (+ _defaultfov 20.0) _returnvalue)
    (`AbilityTask_WaitGameplayTagRemoved.WaitGameplayTagRemove` (struct :`TagName` "Ability.Slide") null
      (:`then`
        (`self.BP_ApplyGameplayEffectToOwner` "/Game/Abilities/GE_Slide.GE_Slide_C"))
      (:`Removed`
        (set `CharacterMovementComponent.GroundFriction` 8.0 (`Character.CharacterMovement` _asbp_player_character))
        (set `PlayerCameraManager.DefaultFOV` (`self.Default FOV`) (`GameplayStatics.GetPlayerCameraManager` 0))
        (`Character.UnCrouch` _asbp_player_character)
        (`self.K2_EndAbility`)))))