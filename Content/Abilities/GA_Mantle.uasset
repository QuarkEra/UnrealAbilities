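; Gameplay ability that performs the player character's mantle as a physics launch.
; On activation it commits, then launches BP_PlayerCharacter along the capsule-to-Box1 offset plus a fixed upward boost, overriding existing velocity.
; It starts waiting for removal of the Ability.Mantle tag, applies GE_Mantle to the owner, and ends when that tag is removed.
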(event `self.K2_ActivateAbility`
  (`parent.K2_ActivateAbility`)
  (bind _asbp_player_character (cast `/Game/Blueprints/BP_PlayerCharacter` (`self.GetOwningActorFromActorInfo`)))
  (`self.K2_CommitAbility`)
  (`Character.LaunchCharacter` _asbp_player_character (+ (- (`SceneComponent.K2_GetComponentLocation` (`/Game/Blueprints/BP_PlayerCharacter.Box1` _asbp_player_character)) (`SceneComponent.K2_GetComponentLocation` (`Character.CapsuleComponent` _asbp_player_character))) (0.0 0.0 500.0)) true true)
  (`AbilityTask_WaitGameplayTagRemoved.WaitGameplayTagRemove` (struct :`TagName` "Ability.Mantle") null
    (:`then`
      (`self.BP_ApplyGameplayEffectToOwner` "/Game/Abilities/GE_Mantle.GE_Mantle_C"))
    (:`Removed`
      (`self.K2_EndAbility`))))